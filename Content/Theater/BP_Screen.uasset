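; Theater screen actor that shows video from a Media Player on a static mesh.
; The construction script gives the mesh a dynamic instance of M_Screen and binds the Sample texture to its texture parameter.
; BeginPlay opens the MS_Sample media source on MPSample.
; Custom events reopen the media or alternate between pause and play through a FlipFlop that pauses first, while a Rewind node is left unconnected.
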(event `self.ReceiveBeginPlay`
  (`MediaPlayer.OpenSource` (`self.MP_Sample`) "/Game/Movies/MS_Sample.MS_Sample"))

(event `PlayandPause`
  (bind _mp_sample (`self.MP_Sample`))
  (`/Engine/EditorBlueprintResources/StandardMacros.FlipFlop`
    (:`A`
      (`MediaPlayer.Pause` _mp_sample))
    (:`B`
      (`MediaPlayer.Play` _mp_sample))))

(event `Reopen`
  (`MediaPlayer.Reopen` (`self.MP_Sample`)))

(fn `UserConstructionScript`
  (bind _returnvalue (`KismetMaterialLibrary.CreateDynamicMaterialInstance` "/Game/Theater/M_Screen.M_Screen"))
  (bind _output_get (set `self.M_Screen_MID` _returnvalue))
  (`PrimitiveComponent.SetMaterial` (`self.StaticMeshComponent`) 0 _output_get)
  (`MaterialInstanceDynamic.SetTextureParameterValue` (`self.M_Screen_MID`) "Sample" (`self.Sample`)))