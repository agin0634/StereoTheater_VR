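; BP_MarkManager is a theater actor that labels the marks of a BP_Mark actor with their coordinates.
; Its construction script takes the first BP_Mark found and adds a text render component for each entry in its Marks array, showing world X and Y.
; Each label uses the mark's world location as its relative location, with a fixed rotation.
; The event graph has no logic.
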(event `self.ReceiveBeginPlay`)

(fn `UserConstructionScript`
  (bind _outactors (`GameplayStatics.GetAllActorsOfClass` "/Game/Theater/BP_Mark.BP_Mark_C"))
  (for _array_element (`/Game/Theater/BP_Mark.Marks` (`|GetArrayItem` _outactors))
    (bind _returnvalue (`SceneComponent.K2_GetComponentLocation` _array_element))
    (bind _returnvalue_2 (`AddComponent|NODE_AddTextRenderComponent-3` :`RelativeTransform` (`KismetMathLibrary.MakeTransform` _returnvalue (struct :`Pitch` 75.0))))
    (`TextRenderComponent.K2_SetText` _returnvalue_2 (`KismetTextLibrary.Conv_StringToText` (`KismetStringLibrary.Concat_StrStr` (`KismetStringLibrary.Conv_DoubleToString` (.x _returnvalue)) "," (`KismetStringLibrary.Conv_DoubleToString` (.y _returnvalue)))))))